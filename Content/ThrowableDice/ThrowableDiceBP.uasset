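; Thrown dice actor that damages actors tagged "Enemy" when its box overlaps them, then destroys itself after a short delay.
; On spawn, the box briefly ignores the Pawn channel before switching to Block.
; Each tick, a short downward trace plus a horizontal speed check detects rolling along a surface and plays a roll sound.
; A DoOnce with a delayed reset throttles that sound.
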(event `self.ReceiveBeginPlay`
  (`PrimitiveComponent.SetCollisionResponseToChannel` (`self.Box`) "ECC_Pawn" "ECR_Ignore")
  (`KismetSystemLibrary.Delay` 0.2)
  (`PrimitiveComponent.SetCollisionResponseToChannel` (`self.Box`) "ECC_Pawn" "ECR_Block"))

(event `self.Box.OnComponentBeginOverlap`
  (params (OverlappedComponent :type "PrimitiveComponent Object Reference") (OtherActor :type "Actor Object Reference") (OtherComp :type "PrimitiveComponent Object Reference") (OtherBodyIndex :type Integer) (bFromSweep :type Boolean) (SweepResult :type "HitResult Structure (by ref)"))
  (if (`self.ActorHasTag` OtherActor "Enemy")
    (`KismetSystemLibrary.Delay` 0.2)
    (`GameplayStatics.ApplyDamage` OtherActor (`self.Damage`) null self)
    (`self.K2_DestroyActor`)))

(event `self.ReceiveTick`
  (params (DeltaSeconds :type "Float (single-precision)"))
  (bind _returnvalue (`self.K2_GetActorLocation`))
  (bind (_outhit _returnvalue_2) (`KismetSystemLibrary.LineTraceSingle` :`Start` _returnvalue :`End` (+ _returnvalue (0.0 0.0 -20.0)) :`TraceChannel` "TraceTypeQuery1" :`DrawDebugType` "ForOneFrame"))
  (if (and (> (`KismetMathLibrary.VSize2D` (`KismetMathLibrary.MakeVector2D` (.x (`self.GetVelocity`)) (.y (`self.GetVelocity`)))) 50.0) _returnvalue_2)
    (`/Engine/EditorBlueprintResources/StandardMacros.DoOnce` false :!label _label
      (:`Completed`
        (`GameplayStatics.PlaySoundAtLocation` "/Game/Blueprints/Characters/Player/Assets/SFX/DiceRoll_Cue.DiceRoll_Cue" (`self.K2_GetActorLocation`) (struct) 1.0 1.0 0.0 null null null null)
        (`KismetSystemLibrary.Delay` 1.6)
        (goto _label :!via `Reset`)))))

(fn `UserConstructionScript`)