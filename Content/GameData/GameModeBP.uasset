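; GameModeBP is a game mode that tracks how many enemies are alive and handles the end-of-round win screen.
; IncreaseEnemies and DecreaseEnemies adjust the EnemiesAlive count.
; NewRound adds a WinScreen widget to the viewport, pauses the game and shows the mouse cursor.
; A MaxEnemies increment is left unconnected, and nothing in this graph checks the enemy count to trigger NewRound.
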(event `New Round`
  (bind _returnvalue (`|CreateWidget` "/Game/Widgets/WinScreen/WinScreen.WinScreen_C"))
  (`UserWidget.AddToViewport` _returnvalue 0)
  (`GameplayStatics.SetGamePaused` true)
  (set `PlayerController.bShowMouseCursor` true (`GameplayStatics.GetPlayerController` 0)))

(event `Increase Enemies`
  (`/Engine/EditorBlueprintResources/StandardMacros.IncrementInt` (`self.Enemies Alive`)))

(event `Decrease Enemies`
  (`/Engine/EditorBlueprintResources/StandardMacros.DecrementInt` (`self.Enemies Alive`)))

(fn `UserConstructionScript`)